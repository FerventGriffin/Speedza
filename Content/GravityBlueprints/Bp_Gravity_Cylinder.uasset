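; Gravity volume actor that pulls physics-simulating objects toward the central axis of a cylinder, giving line-based gravity.
; Each tick, unless GravityOff, it applies an impulse to simulating actors overlapping the Box, aimed at the closest point on the cylinder's up-vector line and scaled by GravityStrength.
; Construction scales the Box from GravityBoundsDimensions and offsets debug handles by reference-object bounds.
; DebugMode shows the cylinder and draws target spheres.
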(event `self.ReceiveBeginPlay`
  ;[1 0 0.152] BeginPlay
  (`|ExecutionSequence`
    (:`then_0`
      (if (`self.DebugMode?`)
        (`KismetSystemLibrary.PrintString` (`KismetStringLibrary.Concat_StrStr` "[" (`KismetSystemLibrary.GetDisplayName` self) "]: " "Awake!") true true (struct :`G` 1.0 :`B` 0.33201 :`A` 1.0) 10.0))
      (`SceneComponent.SetHiddenInGame` (`self.Cylinder`) (not (`self.DebugMode?`)) true))))

(event `self.ReceiveTick`
  (params (DeltaSeconds :type "Float (single-precision)"))
  (bind _cylinder (`self.Cylinder`))
  ;[1 0 0.1803] Gravity Update
  (`|ExecutionSequence`
    (:`then_0`
      (if (not (`self.GravityOff?`))
        (for _array_element (`PrimitiveComponent.GetOverlappingActors` (`self.Box`) "/Script/Engine.Actor")
          (bind _returnvalue (`self.GetComponentByClass` _array_element "/Script/Engine.PrimitiveComponent"))
          (if (and (`SceneComponent.IsSimulatingPhysics` _returnvalue "None") (not (== (`GameplayStatics.GetObjectClass` (`ActorComponent.GetOwner` _returnvalue)) (`GameplayStatics.GetObjectClass` self))))
            (bind _returnvalue_2 (`SceneComponent.K2_GetComponentLocation` _returnvalue))
            (`PrimitiveComponent.AddImpulse` _returnvalue (`self.GetGravityForCylindar` _returnvalue_2) "None" false)
            (if (`self.DebugMode?`)
              (`KismetSystemLibrary.DrawDebugSphere` (`KismetMathLibrary.FindClosestPointOnLine` _returnvalue_2 (`SceneComponent.K2_GetComponentLocation` _cylinder) (`SceneComponent.GetUpVector` _cylinder)) 50.0 12 (struct :`G` 1.0 :`B` 0.960562 :`A` 1.0) 0.03 4.0))))))))

(fn `GetGravityForCylindar`
  (params (`Target Component Location` :type "Vector Structure"))
  (returns (CylindricalGravityDireciton :type "Vector Structure"))
  (bind _cylinder (`self.Cylinder`))
  (return (* (`self.GravityStrength`) (`KismetMathLibrary.Normal` (- (`KismetMathLibrary.FindClosestPointOnLine` `Target Component Location` (`SceneComponent.K2_GetComponentLocation` _cylinder) (`SceneComponent.GetUpVector` _cylinder)) `Target Component Location`)))))

(fn `UserConstructionScript`
  (bind _objectboundsref (`self.ObjectBoundsRef`))
  (bind _returnvalue (* (`KismetMathLibrary.SelectFloat` (.x (`.BoxExtent` (`self.GetActorBounds` _objectboundsref false false))) 500.0 (`KismetSystemLibrary.IsValid` _objectboundsref)) 1.5))
  ;[0.8817 0 1] Construct Graph
  (`|ExecutionSequence`
    (:`then_0`
      (`SceneComponent.SetWorldScale3D` (`self.Box`) (`self.GravityBoundsDimensions`)))
    (:`then_1`
      (`|ExecutionSequence`
        (:`then_0`
          (`SceneComponent.K2_SetRelativeLocation` (`self.Cylinder X1`) (`KismetMathLibrary.MakeVector` _returnvalue) false false)
          (`SceneComponent.K2_SetRelativeLocation` (`self.Cylinder X2`) (`KismetMathLibrary.MakeVector` (* _returnvalue -1.0)) false false)
          (`SceneComponent.K2_SetRelativeLocation` (`self.Cylinder Y1`) (`KismetMathLibrary.MakeVector` 0.0 _returnvalue) false false)
          (`SceneComponent.K2_SetRelativeLocation` (`self.Cylinder Y2`) (`KismetMathLibrary.MakeVector` 0.0 (* _returnvalue -1.0)) false false)
          (`SceneComponent.K2_SetRelativeLocation` (`self.Cylinder Z1`) (`KismetMathLibrary.MakeVector` 0.0 0.0 _returnvalue) false false)
          (`SceneComponent.K2_SetRelativeLocation` (`self.Cylinder Z2`) (`KismetMathLibrary.MakeVector` 0.0 0.0 (* _returnvalue -1.0)) false false))))))