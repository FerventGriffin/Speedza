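; Radial gravity volume centered on a planet that applies impulses to overlapping physics-simulating actors each tick while gravity is on.
; Impulses run along the center-to-actor axis, with strength lerped between minimum and full values by distance from PlanetRef's bounds, and printed each time.
; Construction sizes the overlap sphere from Radius and spaces six axis spheres around the planet's extent.
; DebugMode reveals the main and center spheres at BeginPlay.
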(event `self.ReceiveBeginPlay`
  (bind _returnvalue (not (`self.DebugMode?`)))
  ;[1 0 0.3634] BeginPlay
  ;[0 0 0] Debug Settings
  (`|ExecutionSequence`
    (:`then_0`
      (`SceneComponent.SetHiddenInGame` (`self.Sphere`) _returnvalue false)
      (`SceneComponent.SetHiddenInGame` (`self.Sphere1`) _returnvalue false))))

(event `self.ReceiveTick`
  (params (DeltaSeconds :type "Float (single-precision)"))
  (bind _radius (`self.Radius`))
  (bind _returnvalue (`SceneComponent.K2_GetComponentLocation` (`self.Sphere1`)))
  ;[1 0 0.0231] Gravity Update
  (`|ExecutionSequence`
    (:`then_0`
      (if (not (`self.GravityOff?`))
        (for _array_element (`PrimitiveComponent.GetOverlappingActors` (`self.Sphere`) "/Script/Engine.Actor")
          (bind _returnvalue_2 (`self.GetComponentByClass` _array_element "/Script/Engine.PrimitiveComponent"))
          (if (and (`SceneComponent.IsSimulatingPhysics` _returnvalue_2 "None") (not (== (`GameplayStatics.GetObjectClass` (`ActorComponent.GetOwner` _returnvalue_2)) (`GameplayStatics.GetObjectClass` self))))
            (bind _returnvalue_3 (`self.K2_GetActorLocation` _array_element))
            (bind _returnvalue_4 (`KismetMathLibrary.Lerp` (`self.MinImpulseStrength_Gravity`) (`self.ImpulseStrength_Gravity`) (/ (/ (- (* _radius 10.0) (- (`KismetMathLibrary.Vector_Distance` _returnvalue _returnvalue_3) (.x (`.BoxExtent` (`self.GetActorBounds` (`self.PlanetRef`) false false))))) _radius) 10.0)))
            (`PrimitiveComponent.AddImpulse` _returnvalue_2 (* (`KismetMathLibrary.Normal` (- _returnvalue_3 _returnvalue)) _returnvalue_4) "None" false)
            (`KismetSystemLibrary.PrintString` (`KismetStringLibrary.Conv_DoubleToString` _returnvalue_4) true true (struct :`G` 0.66 :`B` 1.0 :`A` 1.0) 0.01)))))))

(fn `UserConstructionScript`
  (bind _planetref (`self.PlanetRef`))
  (bind _returnvalue (* (`KismetMathLibrary.SelectFloat` (.x (`.BoxExtent` (`self.GetActorBounds` _planetref false false))) 500.0 (`KismetSystemLibrary.IsValid` _planetref)) 1.5))
  ;[0.4375 0.0705 0.2427] Construct Initialize Script
  (`|ExecutionSequence`
    (:`then_0`
      (`SphereComponent.SetSphereRadius` (`self.Sphere`) (`self.Radius`) true)
      (`SceneComponent.K2_SetRelativeLocation` (`self.Sphere X1`) (`KismetMathLibrary.MakeVector` _returnvalue) false false)
      (`SceneComponent.K2_SetRelativeLocation` (`self.Sphere X2`) (`KismetMathLibrary.MakeVector` (* _returnvalue -1.0)) false false)
      (`SceneComponent.K2_SetRelativeLocation` (`self.Sphere Y1`) (`KismetMathLibrary.MakeVector` 0.0 _returnvalue) false false)
      (`SceneComponent.K2_SetRelativeLocation` (`self.Sphere Y2`) (`KismetMathLibrary.MakeVector` 0.0 (* _returnvalue -1.0)) false false)
      (`SceneComponent.K2_SetRelativeLocation` (`self.Sphere Z1`) (`KismetMathLibrary.MakeVector` 0.0 0.0 _returnvalue) false false)
      (`SceneComponent.K2_SetRelativeLocation` (`self.Sphere Z2`) (`KismetMathLibrary.MakeVector` 0.0 0.0 (* _returnvalue -1.0)) false false))))