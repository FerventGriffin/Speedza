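; Directional gravity volume that pushes physics-simulating components overlapping its Box along a configurable direction.
; Every Tick it applies an impulse to each one, skipping actors of its own class, without delta-time scaling.
; The impulse runs from the Cube toward the Arrow, normalized and scaled by GravityStrength.
; On BeginPlay it prints an awake message and uses DebugMode to show or hide the Cube and Arrow.
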(event `self.ReceiveBeginPlay`
  (bind _debug_mode (`self.Debug Mode`))
  ;[1 0 0.4215] Initilize Script
  (`|ExecutionSequence`
    (:`then_0`
      (`KismetSystemLibrary.PrintString` (`KismetStringLibrary.Concat_StrStr` "[" (`KismetSystemLibrary.GetDisplayName` self) "]: " "Awake!") true true (struct :`G` 1.0 :`B` 0.33201 :`A` 1.0) 10.0)
      (`SceneComponent.SetVisibility` (`self.Cube`) _debug_mode false)
      (`SceneComponent.SetHiddenInGame` (`self.Arrow`) (not _debug_mode) false))))

(event `self.ReceiveTick`
  (params (DeltaSeconds :type "Float (single-precision)"))
  ;[0.2217 0 1] Gravity Update
  (`|ExecutionSequence`
    (:`then_0`
      (for _array_element (`PrimitiveComponent.GetOverlappingComponents` (`self.Box`))
        (if (and (`SceneComponent.IsSimulatingPhysics` _array_element "None") (not (== (`GameplayStatics.GetObjectClass` (`ActorComponent.GetOwner` _array_element)) (`GameplayStatics.GetObjectClass` self))))
          (`PrimitiveComponent.AddImpulse` _array_element (`self.GetNewGravityDirection`) "None" false))))))

(fn `GetNewGravityDirection`
  (returns (`Gravity Force` :type "Vector Structure"))
  (return (* (`self.GravityStrength`) (`KismetMathLibrary.Normal` (- (`SceneComponent.K2_GetComponentLocation` (`self.Arrow`)) (`SceneComponent.K2_GetComponentLocation` (`self.Cube`)))))))

(fn `UserConstructionScript`)