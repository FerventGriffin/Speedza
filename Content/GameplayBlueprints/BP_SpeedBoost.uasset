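; BP_SpeedBoost is a boost pad that kicks whatever overlaps its trigger box with a velocity-change impulse.
; The player's SportsCar_Pawn also gains NO2 meter, while other components are boosted only if simulating physics.
; OmniDirectionalBoost selects the target's normalized velocity over the pad's forward vector as impulse direction, and swaps the cube's material at construction.
; DebugMode reveals the arrow and box in game and prints on BeginPlay.
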(event `self.ReceiveTick`
  (params (DeltaSeconds :type "Float (single-precision)"))
  ;[1 0 0.1623] Tick Events
)

(event `self.ReceiveBeginPlay`
  ;[1 0 0.08926] Begin Play
  (if (`self.DebugMode?`)
    (`KismetSystemLibrary.PrintString` (`KismetStringLibrary.Concat_StrStr` "[" (`KismetSystemLibrary.GetDisplayName` self) "]:" "  Awake!") true true (struct :`G` 1.0 :`B` 0.496379 :`A` 1.0) 5.0)))

(event `self.Box.OnComponentBeginOverlap`
  (params (OverlappedComponent :type "PrimitiveComponent Object Reference") (OtherActor :type "Actor Object Reference") (OtherComp :type "PrimitiveComponent Object Reference") (OtherBodyIndex :type Integer) (bFromSweep :type Boolean) (SweepResult :type "HitResult Structure (by ref)"))
  (bind _returnvalue (`ActorComponent.GetOwner` OtherComp))
  ;[1 0 0.05658] Trigger Boost
  (if (== _returnvalue (`GameplayStatics.GetPlayerPawn` 0))
    (bind _assports_car_pawn (cast `/Game/VehicleTemplate/Blueprints/SportsCar/SportsCar_Pawn` _returnvalue))
    (set `/Game/VehicleTemplate/Blueprints/SportsCar/SportsCar_Pawn.NO2 Meter` (+ (`/Game/VehicleTemplate/Blueprints/SportsCar/SportsCar_Pawn.NO2 Meter` _assports_car_pawn) (`self.N02_Meter Refresh`)) _assports_car_pawn)
    (`PrimitiveComponent.AddImpulse` OtherComp (* (`KismetMathLibrary.SelectVector` (`KismetMathLibrary.Normal` (`self.GetVelocity` _returnvalue)) (`self.GetActorForwardVector`) (`self.OmniDirectionalBoost?`)) (`self.ContactBoostStrength`)) "None" true)
    (elif (`SceneComponent.IsSimulatingPhysics` OtherComp "None")
      (`PrimitiveComponent.AddImpulse` OtherComp (* (`KismetMathLibrary.SelectVector` (`KismetMathLibrary.Normal` (`SceneComponent.GetComponentVelocity` OtherComp)) (`self.GetActorForwardVector`) (`self.OmniDirectionalBoost?`)) (`self.ContactBoostStrength`)) "None" true))))

(fn `UserConstructionScript`
  ;[0.2812 0 0.5625] Construct
  (`SceneComponent.SetHiddenInGame` (`self.Arrow Forward`) (not (`self.DebugMode?`)) false)
  (`SceneComponent.SetHiddenInGame` (`self.Box`) (not (`self.DebugMode?`)) false)
  (`PrimitiveComponent.SetMaterial` (`self.Cube`) 0 (select `bool` (not (`self.OmniDirectionalBoost?`)) :`false` "/Game/LevelPrototyping/Materials/MI_PrototypeGrid_TopDark__Inst_Blue.MI_PrototypeGrid_TopDark__Inst_Blue" :`true` "/Game/LevelPrototyping/Materials/MI_PrototypeGrid_TopDark_INst_Orange_Inst_GREEN_Inst.MI_PrototypeGrid_TopDark_INst_Orange_Inst_GREEN_Inst" :!type "MaterialInterface Object Reference")))