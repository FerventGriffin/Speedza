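; BP_BoundsVolume is a play-area boundary volume that tells the game mode when the player enters or leaves the allowed bounds.
; ZoneBoundry overlap events filter for the player pawn and send enter or exit messages.
; Exit fires only when the pawn overlaps no other bounds volume, so overlapping volumes can form one continuous area.
; CallPlayerDeath forwards a death message, and DebugMode makes the boundary visible in game.
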(event `self.ZoneBoundry.OnComponentBeginOverlap`
  (params (OverlappedComponent :type "PrimitiveComponent Object Reference") (OtherActor :type "Actor Object Reference") (OtherComp :type "PrimitiveComponent Object Reference") (OtherBodyIndex :type Integer) (bFromSweep :type Boolean) (SweepResult :type "HitResult Structure (by ref)"))
  ;[1 0.231 0.3408] EndOverlap
  (`|ExecutionSequence`
    (:`then_0`
      (if (`/Game/GameplayBlueprints/BPFL_Speedza.CheckActorEqualsActor` OtherActor (`GameplayStatics.GetPlayerPawn` 0))
        (message `/Game/GameplayBlueprints/GameMode/BPI_SpeedzaGameMode.PlayerEnterBounds` (`GameplayStatics.GetGameMode`))))))

(event `self.ZoneBoundry.OnComponentEndOverlap`
  (params (OverlappedComponent :type "PrimitiveComponent Object Reference") (OtherActor :type "Actor Object Reference") (OtherComp :type "PrimitiveComponent Object Reference") (OtherBodyIndex :type Integer))
  (bind _overlappingactors (`self.GetOverlappingActors` (`GameplayStatics.GetPlayerPawn` 0) "BP_BoundsVolume_C"))
  (bind _returnvalue (`KismetArrayLibrary.Array_Length` _overlappingactors))
  ;[0 0.2438 1] BoundryOverlapCheck
  (`|ExecutionSequence`
    (:`then_0`
      (if (and (`/Game/GameplayBlueprints/BPFL_Speedza.CheckActorEqualsActor` OtherActor (`GameplayStatics.GetPlayerPawn` 0)) (or (not (> _returnvalue 0)) (and (`KismetArrayLibrary.Array_Contains` _overlappingactors self) (<= _returnvalue 1))))
        (message `/Game/GameplayBlueprints/GameMode/BPI_SpeedzaGameMode.PlayerExitBounds` (`GameplayStatics.GetGameMode`))))))

(event `CallPlayerDeath`
  ;[0.01042 1 1] PlayerDeath
  (message `/Game/GameplayBlueprints/GameMode/BPI_SpeedzaGameMode.PlayerDeath` (`GameplayStatics.GetGameMode`)))

(fn `UserConstructionScript`
  ;[0.5214 0 1] Construction Script
  (`|ExecutionSequence`
    (:`then_0`
      (`SceneComponent.SetHiddenInGame` (`self.ZoneBoundry`) (not (`self.DebugMode`)) false))))