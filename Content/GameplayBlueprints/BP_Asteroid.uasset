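; Asteroid projectile with optional homing that trails fire and ends the player's run on contact.
; Spawner-supplied settings and a lifespan configure its ProjectileMovement across the construction script and BeginPlay.
; Sphere overlaps and hits run duplicate detection functions, skipping non-player actors with "volume" in their names.
; Detection spawns an explosion, then a DoOnce-guarded event reports player death to the GameMode and destroys the asteroid, which explodes again on Destroyed.
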(event `/Game/GameplayBlueprints/BPI_Projectile.SetProjectileSettings`
  (params (InitialSpeed :type "Float (double-precision)") (MaxSpeed :type "Float (double-precision)") (`Homing?` :type Boolean) (HomingTarget :type "SceneComponent Object Reference"))
  ;[0 0.2021 1] Set Projectile Actions Up!
  (set `self.ProjectileSpeed_Initial` InitialSpeed)
  (set `self.ProjectileSpeed_Max` MaxSpeed)
  (set `self.IsHoming?` `Homing?`)
  (set `self.TargetedComponent` HomingTarget))

(event `self.ReceiveBeginPlay`
  ;[1 0 0.1564] Innit
  (set `ProjectileMovementComponent.HomingTargetComponent` (`self.TargetedComponent`) (`self.ProjectileMovement`))
  (`GameplayStatics.SpawnEmitterAttached` "/Game/StarterContent/Particles/P_Fire.P_Fire" (`self.StaticMesh`) "None" (0.0 0.0 0.0) (struct) (25.0 25.0 25.0)))

(event `self.Sphere.OnComponentBeginOverlap`
  (params (OverlappedComponent :type "PrimitiveComponent Object Reference") (OtherActor :type "Actor Object Reference") (OtherComp :type "PrimitiveComponent Object Reference") (OtherBodyIndex :type Integer) (bFromSweep :type Boolean) (SweepResult :type "HitResult Structure (by ref)"))
  (bind (_returnvalue_location _returnvalue_rotation _returnvalue_scale) (`KismetMathLibrary.BreakTransform` (`self.GetTransform`)))
  (bind _returnvalue (* _returnvalue_scale 20))
  ;[1 0 0.07651] Detection events
  (`|ExecutionSequence`
    (:`then_0`
      (if (and (!= OtherActor self) (== OtherActor (`GameplayStatics.GetPlayerPawn` 0)))
        (`GameplayStatics.SpawnEmitterAtLocation` "/Game/StarterContent/Particles/P_Explosion.P_Explosion" _returnvalue_location (struct) _returnvalue)
        (`self.TriggerDetected!` true)
        (elif (not (`KismetStringLibrary.Contains` (`KismetSystemLibrary.GetDisplayName` OtherActor) "volume"))
          (`GameplayStatics.SpawnEmitterAtLocation` "/Game/StarterContent/Particles/P_Explosion.P_Explosion" _returnvalue_location (struct) _returnvalue)
          (`self.TriggerDetected!` false))))))

(event `self.Sphere.OnComponentHit`
  (params (HitComponent :type "PrimitiveComponent Object Reference") (OtherActor :type "Actor Object Reference") (OtherComp :type "PrimitiveComponent Object Reference") (NormalImpulse :type "Vector Structure") (Hit :type "HitResult Structure (by ref)"))
  (bind (_returnvalue_location _returnvalue_rotation _returnvalue_scale) (`KismetMathLibrary.BreakTransform` (`self.GetTransform`)))
  (bind _returnvalue (* _returnvalue_scale 20))
  ;[1 0 0.07651] Detection events
  (`|ExecutionSequence`
    (:`then_0`
      (if (and (!= OtherActor self) (== OtherActor (`GameplayStatics.GetPlayerPawn` 0)))
        (`GameplayStatics.SpawnEmitterAtLocation` "/Game/StarterContent/Particles/P_Explosion.P_Explosion" _returnvalue_location (struct) _returnvalue)
        (`self.TriggerDetected!` true)
        (elif (not (`KismetStringLibrary.Contains` (`KismetSystemLibrary.GetDisplayName` OtherActor) "volume"))
          (`GameplayStatics.SpawnEmitterAtLocation` "/Game/StarterContent/Particles/P_Explosion.P_Explosion" _returnvalue_location (struct) _returnvalue)
          (`self.TriggerDetected!` false))))))

(event `TriggerDetected!`
  (params (`HitPlayer?` :type Boolean))
  ;[1 0 0.7079] OnDetected
  (`/Engine/EditorBlueprintResources/StandardMacros.DoOnce` false
    (:`Completed`
      (if `HitPlayer?`
        (message `/Game/GameplayBlueprints/GameMode/BPI_SpeedzaGameMode.PlayerDeath` (`GameplayStatics.GetGameMode`))
        (`self.K2_DestroyActor`)
        (else
          (`self.K2_DestroyActor`))))))

(event `self.ReceiveDestroyed`
  (bind (_returnvalue_location _returnvalue_rotation _returnvalue_scale) (`KismetMathLibrary.BreakTransform` (`self.GetTransform`)))
  ;[1 0.4085 0] DestructionBinding
  (`GameplayStatics.SpawnEmitterAtLocation` "/Game/StarterContent/Particles/P_Explosion.P_Explosion" _returnvalue_location (struct) (* _returnvalue_scale 20)))

(fn `UserConstructionScript`
  (bind _projectilemovement (`self.ProjectileMovement`))
  (set `ProjectileMovementComponent.bIsHomingProjectile` (`self.IsHoming?`) _projectilemovement)
  (set `ProjectileMovementComponent.InitialSpeed` (`self.ProjectileSpeed_Initial`) _projectilemovement)
  (set `ProjectileMovementComponent.MaxSpeed` (`self.ProjectileSpeed_Max`) _projectilemovement)
  (`self.SetLifeSpan` (`self.ProjectileLifespan`)))